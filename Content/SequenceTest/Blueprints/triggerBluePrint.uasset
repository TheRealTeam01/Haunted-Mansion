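; One-shot trigger actor that plays a cutscene featuring Sevarog, then spawns BP_Sevarog at a fixed location.
; The first overlap by any actor starts the Level Sequence, disables player input, reveals the stand-in SequenceSevarog, and hides weapon, flashlight and phase actors with tick off.
; A timer set to the sequence end time reverses this, destroys the stand-in and trigger, and spawns BP_Sevarog inside the restore loop via DoOnce.
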(event Custom|OnFinish_Sequence
  (Actor|DestroyActor (Variables|Default|GetSequenceSevarog))
  (Input|EnableInput (Game|GetPlayerCharacter 0) (Game|GetPlayerController 0))
  (bind _outactors (Actor|GetAllActorsOfClass "/Script/Engine.Actor"))
  (for _array_element _outactors
    (if (Math|Boolean|ORBoolean (Utilities|ClassIsChildOf (Utilities|GetClass _array_element) "/Game/HauntedMansion/Item/Weapon/BP_Weapon.BP_Weapon_C") (Utilities|ClassIsChildOf (Utilities|GetClass _array_element) "/Game/HauntedMansion/Item/Interact/PickUps/BP_FlashLight.BP_FlashLight_C") (Utilities|ClassIsChildOf (Utilities|GetClass _array_element) "/Game/HauntedMansion/Character/Player/BP_Phase.BP_Phase_C"))
      (Rendering|SetActorHiddenInGame _array_element false)
      (Actor|Tick|SetActorTickEnabled _array_element true)
      (Utilities|FlowControl|DoOnce false
        (:Completed
          (Game|SpawnActorfromClass "/Game/HauntedMansion/Character/BP_Sevarog.BP_Sevarog_C" (Math|Transform|MakeTransform "-300.000000,1110.000000,144.403625") "Undefined" "MultiplyWithRoot" 0 0)))))
  (Actor|DestroyActor))

(event Collision|EventActorBeginOverlap
  (params (OtherActor :type Actor%20Object%20Reference))
  (Utilities|FlowControl|DoOnce false
    (:Completed
      (bind _returnvalue (Sequencer|Player|CreateLevelSequencePlayer "/Game/SequenceTest/CutScene/Sequence.Sequence"))
      (Sequencer|Player|Play _returnvalue :!class /Script/MovieScene.MovieSceneSequencePlayer)
      (Utilities|Time|SetTimerbyEvent (delegate Custom|OnFinish_Sequence) (Class|TimeManagementBlueprintLibrary|ToSeconds(QualifiedFrameTime) (Class|MovieSceneSequencePlayer|GetEndTime _returnvalue)))
      (Input|DisableInput (Game|GetPlayerCharacter 0) (Game|GetPlayerController 0))
      (Rendering|SetActorHiddenInGame (Variables|Default|GetSequenceSevarog) false)
      (bind _outactors (Actor|GetAllActorsOfClass "/Script/Engine.Actor"))
      (for _array_element _outactors
        (if (Math|Boolean|ORBoolean (Utilities|ClassIsChildOf (Utilities|GetClass _array_element) "/Game/HauntedMansion/Item/Weapon/BP_Weapon.BP_Weapon_C") (Utilities|ClassIsChildOf (Utilities|GetClass _array_element) "/Game/HauntedMansion/Item/Interact/PickUps/BP_FlashLight.BP_FlashLight_C") (Utilities|ClassIsChildOf (Utilities|GetClass _array_element) "/Game/HauntedMansion/Character/Player/BP_Phase.BP_Phase_C"))
          (Rendering|SetActorHiddenInGame _array_element true)
          (Actor|Tick|SetActorTickEnabled _array_element))))))

(fn ConstructionScript)
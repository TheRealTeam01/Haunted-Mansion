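; BP_TriggerFall is a falling chandelier trap in the haunted mansion, built on a Geometry Collection held static by the construction script.
; Any overlap with its Box enables physics and gravity, then destroys the Box.
; The first hit, gated by DoOnce, damages the BP_Phase player regardless of what was struck and plays a shatter sound.
; It then applies a light-off material and zeroes the first four BP_ChandelierLight actors found in the level.
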(event OnComponentBeginOverlap(Box)
  (params (OverlappedComponent :type Primitive%20Component%20Object%20Reference) (OtherActor :type Actor%20Object%20Reference) (OtherComp :type Primitive%20Component%20Object%20Reference) (OtherBodyIndex :type Integer) (bFromSweep :type Boolean) (SweepResult :type Hit%20Result%20Structure%20%28by%20ref%29))
  (Physics|SetSimulatePhysics (Variables|Default|GetGeometryCollection) true)
  (Physics|SetEnableGravity (Variables|Default|GetGeometryCollection) true)
  (Components|DestroyComponent (Variables|Default|GetBox)))

(event OnComponentHit(GeometryCollection)
  (params (HitComponent :type Primitive%20Component%20Object%20Reference) (OtherActor :type Actor%20Object%20Reference) (OtherComp :type Primitive%20Component%20Object%20Reference) (NormalImpulse :type Vector :default "0, 0, 0") (Hit :type Hit%20Result%20Structure%20%28by%20ref%29))
  (Utilities|FlowControl|DoOnce false
    (:Completed
      (bind _asbp_phase (Utilities|Casting|CastToBP_Phase (Game|GetPlayerCharacter 0)))
      (Game|Damage|ApplyDamage _asbp_phase 7e+01 (Game|GetPlayerController 0) self)
      (Audio|PlaySound2D "/Game/HauntedMansion/Sound/Screaming/684756__supersouper__glassshatterexplode.684756__supersouper__glassshatterexplode" 2.0 1.0 0.0 0 0)
      (Rendering|Material|CreateDynamicMaterialInstance (Variables|Default|GetGeometryCollection) 0 "/Game/SICKA_mansion/Materials/MI_ChandelierLightOff.MI_ChandelierLightOff" "None" :!class /Script/Engine.PrimitiveComponent)
      (bind _outactors (Actor|GetAllActorsOfClass "/Game/HauntedMansion/Item/Interact/TriggerFall/BP_ChandelierLight.BP_ChandelierLight_C"))
      (Rendering|Components|Light|SetIntensity (Variables|/Game/HauntedMansion/Item/Interact/TriggerFall/BP_ChandelierLight.BP_ChandelierLight_C|GetPointLight (Utilities|Array|Get(acopy) _outactors)) 0.0)
      (Rendering|Components|Light|SetIntensity (Variables|/Game/HauntedMansion/Item/Interact/TriggerFall/BP_ChandelierLight.BP_ChandelierLight_C|GetPointLight (Utilities|Array|Get(acopy) _outactors 1)) 0.0)
      (Rendering|Components|Light|SetIntensity (Variables|/Game/HauntedMansion/Item/Interact/TriggerFall/BP_ChandelierLight.BP_ChandelierLight_C|GetPointLight (Utilities|Array|Get(acopy) _outactors 2)) 0.0)
      (Rendering|Components|Light|SetIntensity (Variables|/Game/HauntedMansion/Item/Interact/TriggerFall/BP_ChandelierLight.BP_ChandelierLight_C|GetPointLight (Utilities|Array|Get(acopy) _outactors 3)) 0.0))))

(event Collision|EventActorBeginOverlap
  (params (OtherActor :type Actor%20Object%20Reference)))

(event EventTick
  (params (DeltaSeconds :type Float%20%28single-precision%29)))

(fn ConstructionScript
  (Physics|SetSimulatePhysics (Variables|Default|GetGeometryCollection) false)
  (Physics|SetEnableGravity (Variables|Default|GetGeometryCollection) false))